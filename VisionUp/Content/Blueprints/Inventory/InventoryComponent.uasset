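; Inventory component that stores items in a fixed number of slots and shows them in a HUD widget.
; BeginPlay sizes the slot array, and AddToInventory overwrites the first default (empty) slot with the given content.
; ToggleInventory only creates the window, anchoring it on the ThirdPersonCharacter's HUD canvas.
; RefreshInventoryHUD rebuilds the window by removing any existing one and creating another.
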(event EventBeginPlay
  (CallFunction|PrepareInventory))

(fn ToggleInventory
  (bind _returnvalue (UserInterface|CreateWidget "/Game/Widget/Inventory.Inventory_C" 0 self))
  (Variables|Default|SetInventoryWindow _returnvalue)
  (bind _asthird_person_character (Utilities|Casting|CastToThirdPersonCharacter (Game|GetPlayerCharacter 0)))
  (bind _returnvalue_2 (Class|CanvasPanel|AddChildtoCanvas (Variables|/Game/Widget/MainHUD.MainHUD_C|GetHudCanvas (Variables|/Game/Blueprints/Character/ThirdPersonCharacter.ThirdPersonCharacter_C|GetMainHudWidget _asthird_person_character)) (Variables|Default|GetInventoryWindow)))
  (Class|CanvasPanelSlot|SetAutoSize _returnvalue_2 false)
  (Class|CanvasPanelSlot|SetAlignment _returnvalue_2 "(X=0.000000,Y=1.000000)")
  (Class|CanvasPanelSlot|SetAnchors _returnvalue_2 (Utilities|Struct|MakeAnchors "(X=0.000000,Y=0.700000)" "(X=0.000000,Y=0.700000)"))
  (Class|CanvasPanelSlot|SetPosition _returnvalue_2 (Variables|Default|GetPosition)))

(fn AddtoInventory
  (params (ContentToAdd :type Slot%20Structure%20Structure))
  (bind _slotstructure (Utilities|Struct|MakeSlotStructure "(Name_10_B8121E594FAFD348A809AE91304E907F=NSLOCTEXT(\"[734284B249AC1C21BE816D8F3F0ECDD6]\", \"A23105F44C7F56CDB9E318BC1C3A4DC8\", \"None\"),Class_7_75CDB6FA46222ABD77598A8EFFF5CC72=None,Thumbnail_17_71FF95644E0B43475639A8B986A9E874=None,Durability_26_FA6E1A3047192C2EDC7E94A7235E5FE2=0.000000)"))
  (bind _inventory (Variables|Default|GetInventory))
  (bind _returnvalue (Utilities|Array|FindItem _inventory _slotstructure))
  (bind _returnvalue_2 (>= _returnvalue 0))
  (if _returnvalue_2
    (Utilities|Array|SetArrayElem _inventory _returnvalue ContentToAdd))
  (return _returnvalue_2))

(fn PrepareInventory
  (Utilities|Array|Resize (Variables|Default|GetInventory) (Variables|Default|GetNumberOfSlots)))

(fn RefreshInventoryHUD
  (Variables|Default|GetInventoryWindow
    (:then
      (Widget|RemovefromParent (Variables|Default|GetInventoryWindow))
      (CallFunction|ToggleInventory))
    (:else
      (CallFunction|ToggleInventory))))
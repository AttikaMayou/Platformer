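; ToolComponent manages a ToolInterface widget that can be toggled on and off over the player's main HUD.
; The first toggle lazily creates the widget, passes it the component, and pins it at a fixed position on the ThirdPersonCharacter's HUD canvas.
; Later toggles flip visibility and switch input between UI-only, with focus and mouse lock, and game-only.
; Debug prints report whether widget creation succeeded.
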(fn ToggleWidget
  (bind _returnvalue (Game|GetPlayerController 0))
  (if (Variables|Default|GetInitialized)
    (bind _toolwidget (Variables|Default|GetToolWidget)
      (:then
        (if (Widget|IsVisible _toolwidget)
          (Widget|SetVisibility _toolwidget "Hidden")
          (Input|SetInputModeGameOnly _returnvalue)
          (else
            (Widget|SetVisibility _toolwidget "Visible")
            (Input|SetInputModeUIOnly _returnvalue (Variables|Default|GetToolWidget) "LockAlways"))))
      (:else
        (CallFunction|InitializeWidget :!label _label)))
    (else
      (goto _label))))

(fn InitializeWidget
  (bind _returnvalue (UserInterface|CreateWidget "/Game/Widget/Tool/ToolInterface.ToolInterface_C" (Game|GetPlayerController 0) self))
  (Variables|Default|SetToolWidget _returnvalue)
  (bind _asthird_person_character (Utilities|Casting|CastToThirdPersonCharacter (Game|GetPlayerCharacter 0)))
  (bind _toolwidget (Variables|Default|GetToolWidget)
    (:then
      (Development|PrintString "TOOL WIDGET OK" true true "(R=1.000000,G=0.986602,B=0.378307,A=1.000000)")
      (bind _returnvalue_2 (Class|CanvasPanel|AddChildtoCanvas (Variables|/Game/Widget/MainHUD.MainHUD_C|GetHudCanvas (Variables|/Game/Blueprints/Character/ThirdPersonCharacter.ThirdPersonCharacter_C|GetMainHudWidget _asthird_person_character)) _toolwidget))
      (Class|CanvasPanelSlot|SetAutoSize _returnvalue_2 false)
      (Class|CanvasPanelSlot|SetAlignment _returnvalue_2 "(X=0.000000,Y=1.000000)")
      (Class|CanvasPanelSlot|SetAnchors _returnvalue_2 (Utilities|Struct|MakeAnchors "(X=0.000000,Y=0.000000)" "(X=0.000000,Y=0.000000)"))
      (Class|CanvasPanelSlot|SetPosition _returnvalue_2 "(X=1400.000000,Y=50.000000)")
      (Input|SetInputModeUIOnly (Game|GetPlayerController 0) (Variables|Default|GetToolWidget) "LockAlways")
      (Variables|Default|SetInitialized true)
      (return))
    (:else
      (Development|PrintString "TOO LWIDGET NOT OK" true true "(R=1.000000,G=0.457403,B=0.288558,A=1.000000)"))))
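; Player controller that creates and holds the player's health HUD widgets.
; On BeginPlay it creates the HeartWidget and MainHUD widgets and caches a ThirdPersonCharacter reference, without adding either widget to the viewport here.
; A separate Init function, not called in this Blueprint, passes zero to the character's ModifyHealth and the HUD's UpdateHearts.
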(event EventBeginPlay
  (CallFunction|CreateWidgetsandReferences))

(fn ConstructionScript)

(fn CreateWidgetsandReferences
  (bind _self self)
  (Utilities|FlowControl|Sequence
    (:then_0
      (bind _returnvalue (UserInterface|CreateWidget "/Game/Widget/HeartWidget.HeartWidget_C" _self))
      (Variables|Default|SetHeartWidget _returnvalue))
    (:then_1
      (bind _returnvalue_2 (UserInterface|CreateWidget "/Game/Widget/MainHUD.MainHUD_C" _self))
      (Variables|Default|SetMainHUDWidget _returnvalue_2))
    (:then_2
      (bind _asthird_person_character (Utilities|Casting|CastToThirdPersonCharacter (Game|GetPlayerCharacter 0)))
      (Variables|Default|SetCharacterRef _asthird_person_character))))

(fn Init
  (Default|ModifyHealth (Variables|Default|GetCharacterRef))
  (Default|UpdateHearts (Variables|Default|GetMainHUDWidget)))
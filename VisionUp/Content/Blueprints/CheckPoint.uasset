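; Checkpoint actor that saves the player's location to a save game slot when something overlaps its trigger.
; The overlap event reads the first player's ThirdPersonCharacter location without checking which actor entered, and prints a confirmation message.
; It then writes that location into the existing "Check" slot's SaveGame, or creates a new SaveGame if none exists.
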(event OnComponentBeginOverlap(Trigger)
  (params (OverlappedComponent :type Primitive%20Component%20Object%20Reference) (OtherActor :type Actor%20Object%20Reference) (OtherComp :type Primitive%20Component%20Object%20Reference) (OtherBodyIndex :type Integer) (bFromSweep :type Boolean) (SweepResult :type Hit%20Result%20Structure%20%28by%20ref%29))
  (Utilities|FlowControl|Sequence
    (:then_0
      (bind _asthird_person_character (Utilities|Casting|CastToThirdPersonCharacter (Game|GetPlayerCharacter 0)))
      (Variables|Default|SetPlayerLoc (Transformation|GetActorLocation _asthird_person_character))
      (Development|PrintString "Checkpoint Reached"))
    (:then_1
      (bind _returnvalue (SaveGame|DoesSaveGameExist "Check"))
      (if _returnvalue
        (bind _returnvalue_2 (SaveGame|LoadGamefromSlot "Check"))
        (bind _assave_game (Utilities|Casting|CastToSaveGame _returnvalue_2))
        (Variables|/Game/Blueprints/SaveGame.SaveGame_C|SetPlayerLocation_s _assave_game (Variables|Default|GetPlayerLoc))
        (SaveGame|SaveGametoSlot _assave_game "Check")
        (else
          (bind _returnvalue_3 (SaveGame|CreateSaveGameObject "/Game/Blueprints/SaveGame.SaveGame_C"))
          (Variables|/Game/Blueprints/SaveGame.SaveGame_C|SetPlayerLocation_s _returnvalue_3 (Variables|Default|GetPlayerLoc))
          (SaveGame|SaveGametoSlot _returnvalue_3 "Check"))))))

(event EventBeginPlay)

(event Collision|EventActorBeginOverlap
  (params (OtherActor :type Actor%20Object%20Reference)))

(event EventTick
  (params (DeltaSeconds :type Float%20%28single-precision%29)))

(fn ConstructionScript)
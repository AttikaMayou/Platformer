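; Light trigger Blueprint that lights up when notified of a player jump, if switching on is allowed, then progressively fades out.
; PlayerJumped boosts the point light, resets the timer and re-enters the Tick fade logic.
; Tick lerps current intensity toward zero with a growing, time-based alpha and clamps it.
; SwitchingLights swaps the mesh's second material between two emissive materials based on an intensity threshold.
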(event Custom|SwitchingLights
  (bind _staticmeshcomponent (Variables|Debug|GetStaticMeshComponent))
  ;[0.9907 0.916 1] Swap Material
  (if (> (Variables|/Script/Engine.LightComponentBase|GetIntensity (Variables|Default|GetPointLight)) 5e+01)
    (Rendering|Material|SetMaterial _staticmeshcomponent 1 "/Game/Geometry/Lampadaire/Emissive_Inst.Emissive_Inst")
    (else
      (Rendering|Material|SetMaterial _staticmeshcomponent 1 "/Game/Geometry/Lampadaire/Emissive.Emissive"))))

(event Custom|PlayerJumped
  (params (canSwitchLightOn :type Boolean))
  ;[0.2771 1 0.2115] Player jumped
  ;[0.8863 0.08654 1] Lights on !
  (if canSwitchLightOn
    (Rendering|Components|Light|SetIntensity (Variables|Default|GetPointLight) 6e+03)
    (CallFunction|SwitchingLights)
    (Variables|Default|SetCurrentTime 0.0)
    ;[0.05151 0.01986 0.3635] Progressive light off
    (bind _output_get (Variables|Default|SetCurrentTime (+ (stale EventTick DeltaSeconds) (Variables|Default|GetCurrentTime))))
    (if (< (Math|Float|Clamp(Float) (Math|Float|Lerp (Variables|/Script/Engine.LightComponentBase|GetIntensity (Variables|Default|GetPointLight)) 0.0 (/ _output_get 3e+01)) 0.0 5e+03) 5e+01)
      (CallFunction|SwitchingLights))
    (Rendering|Components|Light|SetIntensity (Variables|Default|GetPointLight) (Math|Float|Clamp(Float) (Math|Float|Lerp (Variables|/Script/Engine.LightComponentBase|GetIntensity (Variables|Default|GetPointLight)) 0.0 (/ _output_get 3e+01)) 0.0 5e+03))))

(event EventTick
  (params (DeltaSeconds :type Float%20%28single-precision%29))
  ;[0.05151 0.01986 0.3635] Progressive light off
  (bind _output_get (Variables|Default|SetCurrentTime (+ DeltaSeconds (Variables|Default|GetCurrentTime))))
  (if (< (Math|Float|Clamp(Float) (Math|Float|Lerp (Variables|/Script/Engine.LightComponentBase|GetIntensity (Variables|Default|GetPointLight)) 0.0 (/ _output_get 3e+01)) 0.0 5e+03) 5e+01)
    (CallFunction|SwitchingLights))
  (Rendering|Components|Light|SetIntensity (Variables|Default|GetPointLight) (Math|Float|Clamp(Float) (Math|Float|Lerp (Variables|/Script/Engine.LightComponentBase|GetIntensity (Variables|Default|GetPointLight)) 0.0 (/ _output_get 3e+01)) 0.0 5e+03)))

(fn ConstructionScript)